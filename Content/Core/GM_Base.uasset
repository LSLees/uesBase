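; Base game mode that routes player login and logout by level name and runs the ready-up flow in the Lobby.
; A map tracks each player's ready state; once all are ready, a three-second chat countdown rechecks every second, cancelling or server-traveling to Testing through the game instance.
; System messages are broadcast to every PC_Base player controller.
; Login and logout handlers for non-lobby levels are empty stubs.
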(event Custom|BroadcastMSG
  (params (From :type String) (Body :type String))
  (bind _returnvalue (Class|GameModeBase|GetNumPlayers))
  (for _index (range 0 (- _returnvalue 0))
    (bind _aspc_base (Utilities|Casting|CastToPC_Base (Game|GetPlayerController _index)))
    (Default|NewMSG _aspc_base From Body)))

(event EventPostLogin
  (params (NewPlayer :type Player%20Controller%20Object%20Reference))
  (bind _returnvalue (Game|GetCurrentLevelName true))
  (switch string _returnvalue
    (:Default
      (CallFunction|GameLogin))
    (:Lobby
      (CallFunction|LobbyLogin NewPlayer))))

(event EventOnLogout
  (params (ExitingController :type Controller%20Object%20Reference))
  (bind _returnvalue (Game|GetCurrentLevelName true))
  (switch string _returnvalue
    (:Default
      (CallFunction|GameLogout))
    (:Lobby
      (CallFunction|LobbyLogout ExitingController))))

(event Custom|LobbyLogin
  (params (Player :type Controller%20Object%20Reference%20%28by%20ref%29))
  (Utilities|Map|Add (Variables|Default|GetLobbyReadys) Player false))

(event Custom|LobbyLogout
  (params (Player :type Controller%20Object%20Reference%20%28by%20ref%29))
  (Utilities|Map|Remove (Variables|Default|GetLobbyReadys) Player)
  (if (!= (Utilities|Map|Length (Variables|Default|GetLobbyReadys)) 0)
    (CallFunction|CheckReadys)))

(event Custom|CheckReadys
  (bind _values (Utilities|Map|Values (Variables|Default|GetLobbyReadys)))
  (if (not (Utilities|Array|ContainsItem _values false))
    (CallFunction|BroadcastMSG "SYSTEM" "3")
    (Utilities|FlowControl|Delay 1.0)
    (bind _values_2 (Utilities|Map|Values (Variables|Default|GetLobbyReadys)))
    (if (Utilities|Array|ContainsItem _values_2 false)
      (CallFunction|BroadcastMSG "SYSTEM" "Cancelled")
      (else
        (CallFunction|BroadcastMSG "SYSTEM" "2")
        (Utilities|FlowControl|Delay 1.0)
        (bind _values_3 (Utilities|Map|Values (Variables|Default|GetLobbyReadys)))
        (if (Utilities|Array|ContainsItem _values_3 false)
          (CallFunction|BroadcastMSG "SYSTEM" "Cancelled")
          (else
            (CallFunction|BroadcastMSG "SYSTEM" "1")
            (Utilities|FlowControl|Delay 1.0)
            (bind _values_4 (Utilities|Map|Values (Variables|Default|GetLobbyReadys)))
            (if (Utilities|Array|ContainsItem _values_4 false)
              (CallFunction|BroadcastMSG "SYSTEM" "Cancelled")
              (else
                (bind _asinstance (Utilities|Casting|CastToInstance (Game|GetGameInstance)))
                (Default|ServerTravel _asinstance "Testing")))))))))

(event Custom|SetReady
  (params (Player :type Controller%20Object%20Reference) (Ready :type Boolean))
  (Utilities|Map|Add (Variables|Default|GetLobbyReadys) Player Ready)
  (CallFunction|CheckReadys))

(event Custom|GameLogin)

(event Custom|GameLogout)

(fn ConstructionScript)