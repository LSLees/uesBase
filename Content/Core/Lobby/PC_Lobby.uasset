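; PC_Lobby is a player controller that opens the front-end UI for the menu and lobby levels.
; On BeginPlay, the local controller switches to UI-only input and shows the mouse cursor.
; It then switches on the current level name, adding UW_Menu to the viewport for Main Menu and UW_Lobby for Lobby or any other level.
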(event EventBeginPlay
  (if (Pawn|IsLocalPlayerController)
    (Input|SetInputModeUIOnly self 0 "DoNotLock" true)
    (Variables|Default|SetbShowMouseCursor true)
    (bind _returnvalue (Game|GetCurrentLevelName true))
    (switch string _returnvalue
      (:Default
        (bind _returnvalue_2 (UserInterface|CreateWidget "/Game/Widgets/Lobby/UW_Lobby.UW_Lobby_C" :!label _label))
        (UserInterface|Viewport|AddtoViewport _returnvalue_2 0))
      (:MainMenu
        (bind _returnvalue_3 (UserInterface|CreateWidget "/Game/Widgets/Menu/UW_Menu.UW_Menu_C"))
        (UserInterface|Viewport|AddtoViewport _returnvalue_3 0))
      (:Lobby
        (goto _label)))))

(fn ConstructionScript
  (|CallParentFunction))