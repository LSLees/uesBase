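; Base player controller that sets up input, UI and pawns for the main menu, lobby and match, branching on level name at BeginPlay.
; SpawnPlayer possesses a new pawn at the first free BP_SpawnSpot, carrying the player's IGN.
; Death frees a random taken spot, retargets spectators to the killer, spectates them, then respawns after a delay.
; It also relays chat, lobby readiness, scoreboard, pause and end-game AXP, with debug AXP keys.
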(event Custom|NewMSG
  (params (From :type String) (Body :type String) (Colour :type Linear%20Color%20Structure))
  (bind _ashud_base (Utilities|Casting|CastToHUD_Base (HUD|GetHUD)))
  (Default|NewMSG (Variables|/Game/Widgets/HUD_Base.HUD_Base_C|GetLog _ashud_base) From Body Colour))

(event Custom|SpawnPlayer
  (params (ClassOverride :type Player%20Class%20Reference))
  (bind _returnvalue (Pawn|GetControlledPawn))
  (Utilities|FlowControl|Sequence
    (:then_0
      (Utilities|IsValid _returnvalue
        (:Is%20Valid
          (Actor|DestroyActor _returnvalue))))
    (:then_1
      (bind _outactors (Actor|GetAllActorsOfClass "/Game/Game/BP_SpawnSpot.BP_SpawnSpot_C"))
      (bind _array_element (Utilities|Array|ForEachLoopwithBreak _outactors :!label _label)
        (:LoopBody
          (if (not (Variables|/Game/Game/BP_SpawnSpot.BP_SpawnSpot_C|GetTaken _array_element))
            (Utilities|FlowControl|Sequence
              (:then_0
                (goto _label Break))
              (:then_1
                (Variables|/Game/Game/BP_SpawnSpot.BP_SpawnSpot_C|SetTaken _array_element true)
                (bind _asps_base (Utilities|Casting|CastToPS_Base (Variables|GetPlayerState)))
                (bind _asplayer (Utilities|Casting|CastToPlayerClass (select (Utilities|IsValidClass ClassOverride) ClassOverride (Variables|/Game/Core/PS_Base.PS_Base_C|GetClass _asps_base))))
                (bind _returnvalue_2 (Game|SpawnActorfromClass _asplayer (Transformation|GetActorTransform _array_element) "AdjustIfPossibleButAlwaysSpawn" "MultiplyWithRoot" 0 0))
                (Variables|/Game/Player/Player.Player_C|SetIGN _returnvalue_2 (Variables|/Game/Core/PS_Base.PS_Base_C|GetIGN _asps_base))
                (Pawn|Possess _returnvalue_2)
                (CallFunction|CreateUI)))))))))

(event Custom|SetUserInfo
  (params (SteamID :type SIK%20Steam%20Id%20Structure) (IGN :type String))
  (bind _asps_base (Utilities|Casting|CastToPS_Base (Variables|GetPlayerState)))
  (Variables|/Game/Core/PS_Base.PS_Base_C|SetIGN _asps_base IGN))

(event Custom|CreateUI
  (bind _ashud_base (Utilities|Casting|CastToHUD_Base (HUD|GetHUD)))
  (Default|OwnerSpawned _ashud_base))

(event Custom|BroadcastMSG
  (params (Body :type String) (Colour :type Linear%20Color%20Structure))
  (bind _asgm_base (Utilities|Casting|CastToGM_Base (Game|GetGameMode)))
  (bind _asps_base (Utilities|Casting|CastToPS_Base (Variables|GetPlayerState)))
  (Default|BroadcastMSG _asgm_base (Variables|/Game/Core/PS_Base.PS_Base_C|GetIGN _asps_base) Body Colour))

(event EventTick
  (params (DeltaSeconds :type Float%20%28single-precision%29)))

(event EventBeginPlay
  (if (Pawn|IsLocalPlayerController)
    (Class|WidgetBlueprintLibrary|SetFocustoGameViewport)
    (bind _returnvalue (Game|GetCurrentLevelName true))
    (switch string _returnvalue
      (:Default
        (CallFunction|GameSpawn))
      (:MainMenu
        (CallFunction|LobbySpawn :!label _label))
      (:Lobby
        (goto _label)))))

(event Custom|SetReady
  (params (Ready? :type Boolean))
  (bind _asgm_base (Utilities|Casting|CastToGM_Base (Game|GetGameMode)))
  (Default|SetReady _asgm_base self Ready?)
  (bind _aslobby (Utilities|Casting|CastToLobby (Pawn|GetControlledPawn)))
  (Variables|/Game/Player/Lobby.Lobby_C|SetReady? _aslobby Ready?))

(event Custom|LobbyEnd
  (bind _asinstance (Utilities|Casting|CastToInstance (Game|GetGameInstance)))
  (Variables|/Game/Core/Instance.Instance_C|SetLobbyID _asinstance "")
  (Game|OpenLevel(byObjectReference) "/Game/Levels/MainMenu.MainMenu"))

(event Custom|LobbySpawn
  (bind _returnvalue (PlayerController|LocalPlayerSubsystems|GetEnhancedInputLocalPlayerSubsystem))
  (Utilities|IsValid _returnvalue
    (:Is%20Valid
      (Input|AddMappingContext _returnvalue "/Game/Input/IMC_Main.IMC_Main" 0 "(bIgnoreAllPressedKeysUntilRelease=True,bForceImmediately=False,bNotifyUserSettings=False)")
      (Input|SetInputModeUIOnly self 0 "DoNotLock" true)
      (Variables|Default|SetbShowMouseCursor true)
      (bind _returnvalue_2 (Game|GetCurrentLevelName true))
      (switch string _returnvalue_2
        (:Default
          (bind _returnvalue_3 (UserInterface|CreateWidget "/Game/Widgets/Menu/UW_Menu.UW_Menu_C"))
          (UserInterface|Viewport|AddtoViewport _returnvalue_3 0))
        (:Lobby
          (bind _ashud_base (Utilities|Casting|CastToHUD_Base (HUD|GetHUD)))
          (Default|MakeLobby _ashud_base)
          (bind _asinstance (Utilities|Casting|CastToInstance (Game|GetGameInstance)))
          (CallFunction|SetUserInfo (Variables|/Game/Core/Instance.Instance_C|GetSteamID _asinstance) (Variables|/Game/Core/Instance.Instance_C|GetSteamName _asinstance))
          (CallFunction|SpawnPlayer "/Game/Player/Lobby.Lobby_C"))))))

(event Custom|Death
  (params (Spectate? :type Boolean) (Killer :type Actor%20Object%20Reference))
  (CallFunction|EnableRandomSpawn)
  (bind _outactors (Actor|GetAllActorsOfClass "/Game/Player/Spectator.Spectator_C"))
  (for _array_element _outactors
    (if (== (Variables|/Game/Player/Spectator.Spectator_C|GetSpectating _array_element) (Pawn|GetControlledPawn))
      (Variables|/Game/Player/Spectator.Spectator_C|SetSpectating _array_element Killer)))
  (CallFunction|Spectate Killer)
  (Utilities|FlowControl|Delay 4.0)
  (CallFunction|SpawnPlayer))

(event Custom|GameEnd
  (params (AXP :type Integer))
  (Input|SetInputModeUIOnly self 0 "DoNotLock" true)
  (Variables|Default|SetbShowMouseCursor true)
  (bind _ashud_base (Utilities|Casting|CastToHUD_Base (HUD|GetHUD)))
  (Default|GameEnd (Variables|/Game/Widgets/HUD_Base.HUD_Base_C|GetHUD _ashud_base))
  (CallFunction|AwardAXP AXP))

(event Custom|GameSpawn
  (bind _returnvalue (PlayerController|LocalPlayerSubsystems|GetEnhancedInputLocalPlayerSubsystem))
  (Utilities|IsValid _returnvalue
    (:Is%20Valid
      (Input|AddMappingContext _returnvalue "/Game/Input/IMC_Main.IMC_Main" 0 "(bIgnoreAllPressedKeysUntilRelease=True,bForceImmediately=False,bNotifyUserSettings=False)")
      (Input|SetInputModeGameOnly self true)
      (Variables|Default|SetbShowMouseCursor false)
      (bind _asinstance (Utilities|Casting|CastToInstance (Game|GetGameInstance)))
      (CallFunction|SetUserInfo (Variables|/Game/Core/Instance.Instance_C|GetSteamID _asinstance) (Variables|/Game/Core/Instance.Instance_C|GetSteamName _asinstance))
      (CallFunction|SpawnPlayer "/Game/Player/Player.Player_C"))))

(event Input|EnhancedActionEvents|EnhancedInputActionIA_Board
  (params (ActionValue :type Boolean) (ElapsedSeconds :type Float%20%28double-precision%29) (TriggeredSeconds :type Float%20%28double-precision%29) (InputAction :type Input%20Action%20Object%20Reference :default "/Game/Input/IA_Board.IA_Board"))
  (:Started
    (Class|BPIHUD|ToggleBoard(Message) (HUD|GetHUD) true))
  (:Canceled
    (Class|BPIHUD|ToggleBoard(Message) (HUD|GetHUD) false :!label _label))
  (:Completed
    (goto _label)))

(event Input|EnhancedActionEvents|EnhancedInputActionIA_Pause
  (params (ActionValue :type Boolean) (ElapsedSeconds :type Float%20%28double-precision%29) (TriggeredSeconds :type Float%20%28double-precision%29) (InputAction :type Input%20Action%20Object%20Reference :default "/Game/Input/IA_Pause.IA_Pause"))
  (:Started
    (Class|BPIHUD|TogglePause(Message) (HUD|GetHUD))))

(event Input|KeyboardEvents|DebugKeyJ
  (params (Key :type Key%20Structure) (ActionValue :type Input%20Action%20Value%20Structure))
  (:Pressed
    (CallFunction|AwardAXP 10)))

(event Input|KeyboardEvents|DebugKeyK
  (params (Key :type Key%20Structure) (ActionValue :type Input%20Action%20Value%20Structure))
  (:Pressed
    (CallFunction|AwardAXP 100)))

(fn ConstructionScript)

(fn Spectate
  (params (Who? :type Actor%20Object%20Reference))
  (bind _returnvalue (Game|SpawnActorfromClass "/Game/Player/Spectator.Spectator_C" (Transformation|GetActorTransform (Pawn|GetControlledPawn)) "AdjustIfPossibleButAlwaysSpawn" "MultiplyWithRoot" self Who? 0))
  (Actor|DestroyActor (Pawn|GetControlledPawn))
  (Pawn|Possess _returnvalue)
  (return))

(fn EnableRandomSpawn
  (bind _outactors (Actor|GetAllActorsOfClass "/Game/Game/BP_SpawnSpot.BP_SpawnSpot_C"))
  (for _array_element _outactors
    (if (Variables|/Game/Game/BP_SpawnSpot.BP_SpawnSpot_C|GetTaken _array_element)
      (Utilities|Array|Add (LocalVariables|GetTakens) _array_element)))
  (Variables|/Game/Game/BP_SpawnSpot.BP_SpawnSpot_C|SetTaken (.OutItem (Utilities|Array|Random (LocalVariables|GetTakens))) false)
  (return))